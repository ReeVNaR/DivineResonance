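; Mini-boss AI character that roams random reachable points, chases pawns it sees and attacks in melee.
; Pawn sensing raises walk speed and starts the chase, with a retriggerable delay resuming roaming.
; Attacks are DoOnce-gated, freezing movement during a random montage.
; Montage notifies trigger a sphere overlap on WorldStatic objects, calling ApplyDamage per hit without a damaged actor wired.
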(event `self.ReceiveBeginPlay`
  (`self.Roaming`))

(event `Roaming`
  (`|AIMoveTo` self (`NavigationSystemV1.K2_GetRandomReachablePointInRadius` (`SceneComponent.K2_GetComponentLocation` (`self.Mesh`)) 1000.0 null null) null
    (:`OnSuccess`
      (`KismetSystemLibrary.Delay` (`KismetMathLibrary.RandomFloatInRange` 1.0 4.0))
      (`self.Roaming`))))

(event `Deal Damage`
  (bind _outactors (`KismetSystemLibrary.SphereOverlapActors` (`SceneComponent.K2_GetComponentLocation` (`self.Sphere`)) (`self.AttackRange`) (`|MakeArray` "ObjectTypeQuery1" :!type "EObjectTypeQuery Enum") "/Script/Engine.Actor"))
  (for _ _outactors
    (`GameplayStatics.ApplyDamage` null (`self.Base Damage`) (`self.GetController`) self "/Script/Engine.DamageType")))

(event `self.PawnSensing.OnSeePawn`
  (params (Pawn :type "Pawn Object Reference"))
  (`|ExecutionSequence`
    (:`then_0`
      (set `CharacterMovementComponent.MaxWalkSpeed` 400.0 (`self.CharacterMovement`))
      (`|AIMoveTo` self (0.0 0.0 0.0) Pawn 150.0
        (:`OnSuccess`
          (`self.Attack`))))
    (:`then_1`
      (`KismetSystemLibrary.RetriggerableDelay` 3.0)
      (`self.Roaming`))))

(event `Attack`
  (bind _attackanims (`self.AttackAnims`))
  (`/Engine/EditorBlueprintResources/StandardMacros.DoOnce` false :!label _label
    (:`Completed`
      (`CharacterMovementComponent.DisableMovement` (`self.CharacterMovement`))
      (`|PlayMontage` (`self.Mesh`) (`|GetArrayItem` _attackanims (`KismetMathLibrary.RandomInteger` (`KismetArrayLibrary.Array_Length` _attackanims)))
        (:`then`
          (`GameplayStatics.PlaySound2D` null 1.0 1.0 0.0 null null))
        (:`OnCompleted`
          (`CharacterMovementComponent.SetMovementMode` (`self.CharacterMovement`) "MOVE_Walking" 0 :!label _label_2)
          (goto _label :!via `Reset`))
        (:`OnInterrupted`
          (`KismetSystemLibrary.RetriggerableDelay` 1.0)
          (goto _label_2))
        (:`OnNotifyBegin`
          (`self.Deal Damage`))))))

(fn `UserConstructionScript`)